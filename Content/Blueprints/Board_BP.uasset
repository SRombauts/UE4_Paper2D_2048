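; Board Blueprint for an unfinished 2048-style game on a 4x4 grid stored as a flat 16-cell array.
; On start and on Up, Down or Left, a seeded random stream picks an empty cell for a new 2, drawn as a Paper sprite via index-to-transform helpers.
; Right is experimental, scanning one row and only logging a possible move before spawning.
; A full board simply quits the game.
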(event EventBeginPlay
  (bind _random (Variables|Default|GetRandom))
  (bind _returnvalue (Math|Random|RandomIntegerinRangefromStream 0 15 _random))
  ;[1 1 1] Init Game
  (Utilities|Array|Resize (Variables|Default|GetArray) 16)
  (Class|KismetMathLibrary|SeedRandomStream _random)
  (Input|EnableInput (Game|GetPlayerController 0))
  ;[1 1 1] Add New Number to the Board
  (bind _output_get (Variables|Default|SetIdx _returnvalue))
  (while (> (Utilities|Array|Get(acopy) (Variables|Default|GetArray) _output_get) 0)
    (Variables|Default|SetIdx _returnvalue))
  (Utilities|Array|SetArrayElem (Variables|Default|GetArray) (Variables|Default|GetIdx) 2)
  (Math|Integer|IncrementInt (Variables|Default|GetCount)
    (:%20%20
      (bind (_x _z) (CallFunction|1Dto2D (Variables|Default|GetIdx)))
      (bind _transform (CallFunction|2DtoTransform _x _z))
      (AddComponent|AddPaperSpriteComponent false _transform)
      ;[1 1 1] Debug Print
      (Development|PrintString (Utilities|String|ToString(Text) (Utilities|Text|FormatText "{Count}: {Idx}=[{X},{Z}]" (Utilities|Text|ToText(Integer) (Variables|Default|GetCount)) (Utilities|Text|ToText(Integer) (Variables|Default|GetIdx)) (Utilities|Text|ToText(Integer) _x) (Utilities|Text|ToText(Integer) _z))))
      ;[1 0 0] TODO: proper Game Over
      (if (not (< (Variables|Default|GetCount) 16))
        (Game|QuitGame 0 "Quit")))))

(event Input|ActionEvents|InputActionUp
  (bind _random (Variables|Default|GetRandom))
  (bind _returnvalue (Math|Random|RandomIntegerinRangefromStream 0 15 _random))
  ;[1 0 0] TODO: inputs
  (:Pressed
    (Development|PrintString "Up")
    ;[1 1 1] Add New Number to the Board
    (bind _output_get (Variables|Default|SetIdx _returnvalue))
    (while (> (Utilities|Array|Get(acopy) (Variables|Default|GetArray) _output_get) 0)
      (Variables|Default|SetIdx _returnvalue))
    (Utilities|Array|SetArrayElem (Variables|Default|GetArray) (Variables|Default|GetIdx) 2)
    (Math|Integer|IncrementInt (Variables|Default|GetCount)
      (:%20%20
        (bind (_x _z) (CallFunction|1Dto2D (Variables|Default|GetIdx)))
        (bind _transform (CallFunction|2DtoTransform _x _z))
        (AddComponent|AddPaperSpriteComponent false _transform)
        ;[1 1 1] Debug Print
        (Development|PrintString (Utilities|String|ToString(Text) (Utilities|Text|FormatText "{Count}: {Idx}=[{X},{Z}]" (Utilities|Text|ToText(Integer) (Variables|Default|GetCount)) (Utilities|Text|ToText(Integer) (Variables|Default|GetIdx)) (Utilities|Text|ToText(Integer) _x) (Utilities|Text|ToText(Integer) _z))))
        ;[1 0 0] TODO: proper Game Over
        (if (not (< (Variables|Default|GetCount) 16))
          (Game|QuitGame 0 "Quit"))))))

(event Input|ActionEvents|InputActionDown
  (bind _random (Variables|Default|GetRandom))
  (bind _returnvalue (Math|Random|RandomIntegerinRangefromStream 0 15 _random))
  ;[1 0 0] TODO: inputs
  (:Pressed
    (Development|PrintString "Down")
    ;[1 1 1] Add New Number to the Board
    (bind _output_get (Variables|Default|SetIdx _returnvalue))
    (while (> (Utilities|Array|Get(acopy) (Variables|Default|GetArray) _output_get) 0)
      (Variables|Default|SetIdx _returnvalue))
    (Utilities|Array|SetArrayElem (Variables|Default|GetArray) (Variables|Default|GetIdx) 2)
    (Math|Integer|IncrementInt (Variables|Default|GetCount)
      (:%20%20
        (bind (_x _z) (CallFunction|1Dto2D (Variables|Default|GetIdx)))
        (bind _transform (CallFunction|2DtoTransform _x _z))
        (AddComponent|AddPaperSpriteComponent false _transform)
        ;[1 1 1] Debug Print
        (Development|PrintString (Utilities|String|ToString(Text) (Utilities|Text|FormatText "{Count}: {Idx}=[{X},{Z}]" (Utilities|Text|ToText(Integer) (Variables|Default|GetCount)) (Utilities|Text|ToText(Integer) (Variables|Default|GetIdx)) (Utilities|Text|ToText(Integer) _x) (Utilities|Text|ToText(Integer) _z))))
        ;[1 0 0] TODO: proper Game Over
        (if (not (< (Variables|Default|GetCount) 16))
          (Game|QuitGame 0 "Quit"))))))

(event Input|ActionEvents|InputActionLeft
  (bind _random (Variables|Default|GetRandom))
  (bind _returnvalue (Math|Random|RandomIntegerinRangefromStream 0 15 _random))
  ;[1 0 0] TODO: inputs
  (:Pressed
    (Development|PrintString "Left")
    ;[1 1 1] Add New Number to the Board
    (bind _output_get (Variables|Default|SetIdx _returnvalue))
    (while (> (Utilities|Array|Get(acopy) (Variables|Default|GetArray) _output_get) 0)
      (Variables|Default|SetIdx _returnvalue))
    (Utilities|Array|SetArrayElem (Variables|Default|GetArray) (Variables|Default|GetIdx) 2)
    (Math|Integer|IncrementInt (Variables|Default|GetCount)
      (:%20%20
        (bind (_x _z) (CallFunction|1Dto2D (Variables|Default|GetIdx)))
        (bind _transform (CallFunction|2DtoTransform _x _z))
        (AddComponent|AddPaperSpriteComponent false _transform)
        ;[1 1 1] Debug Print
        (Development|PrintString (Utilities|String|ToString(Text) (Utilities|Text|FormatText "{Count}: {Idx}=[{X},{Z}]" (Utilities|Text|ToText(Integer) (Variables|Default|GetCount)) (Utilities|Text|ToText(Integer) (Variables|Default|GetIdx)) (Utilities|Text|ToText(Integer) _x) (Utilities|Text|ToText(Integer) _z))))
        ;[1 0 0] TODO: proper Game Over
        (if (not (< (Variables|Default|GetCount) 16))
          (Game|QuitGame 0 "Quit"))))))

(event Input|ActionEvents|InputActionRight
  (bind _random (Variables|Default|GetRandom))
  (bind _returnvalue (Math|Random|RandomIntegerinRangefromStream 0 15 _random))
  ;[1 0 0] TODO: inputs
  (:Pressed
    (Development|PrintString "Right")
    ;[1 1 1] Experimental move Right
    (Variables|Default|SetSavedValid false)
    (bind _output_get (Variables|Default|SetZ 3))
    (for _index (range 0 3)
      (bind _idx (CallFunction|2Dto1D _index _output_get))
      (if (Variables|Default|GetSavedValid)
        (if (> (Utilities|Array|Get(acopy) (Variables|Default|GetArray) _idx) 0)
          (if (or (== (Utilities|Array|Get(acopy) (Variables|Default|GetArray) _idx) (Variables|Default|GetSavedVal)) (== (Variables|Default|GetSavedVal) 0))
            (Development|PrintString (Utilities|String|ToString(Text) (Utilities|Text|FormatText "Move Right [{X},{Z}] to [{Xsav},{Zsav}]" (Utilities|Text|ToText(Integer) (Variables|Default|GetSavedX)) (Utilities|Text|ToText(Integer) _index) (Utilities|Text|ToText(Integer) (Variables|Default|GetSavedZ)) (Utilities|Text|ToText(Integer) _output_get))))
            (Variables|Default|SetSavedValid false)
            ;[1 1 1] Add New Number to the Board
            (bind _output_get_2 (Variables|Default|SetIdx _returnvalue))
            (while (> (Utilities|Array|Get(acopy) (Variables|Default|GetArray) _output_get_2) 0)
              (Variables|Default|SetIdx _returnvalue))
            (Utilities|Array|SetArrayElem (Variables|Default|GetArray) (Variables|Default|GetIdx) 2)
            (Math|Integer|IncrementInt (Variables|Default|GetCount)
              (:%20%20
                (bind (_x _z) (CallFunction|1Dto2D (Variables|Default|GetIdx)))
                (bind _transform (CallFunction|2DtoTransform _x _z))
                (AddComponent|AddPaperSpriteComponent false _transform)
                ;[1 1 1] Debug Print
                (Development|PrintString (Utilities|String|ToString(Text) (Utilities|Text|FormatText "{Count}: {Idx}=[{X},{Z}]" (Utilities|Text|ToText(Integer) (Variables|Default|GetCount)) (Utilities|Text|ToText(Integer) (Variables|Default|GetIdx)) (Utilities|Text|ToText(Integer) _x) (Utilities|Text|ToText(Integer) _z))))
                ;[1 0 0] TODO: proper Game Over
                (if (not (< (Variables|Default|GetCount) 16))
                  (Game|QuitGame 0 "Quit"))))
            (else
              (Variables|Default|SetSavedValid true :!label _label)
              (Variables|Default|SetSavedX _index)
              (Variables|Default|SetSavedZ _output_get)
              (Variables|Default|SetSavedCell _idx)
              (Variables|Default|SetSavedVal (Utilities|Array|Get(acopy) (Variables|Default|GetArray) _idx)))))
        (else
          (goto _label))))))

(event Input|ActionEvents|InputActionQuit
  ;[1 1 1] Quit Game
  (:Pressed
    (Game|QuitGame 0 "Quit")))

(fn ConstructionScript)

(fn 1Dto2D
  (params (Idx :type Integer))
  (return (Math|Integer|%(Integer) Idx 4) (/ Idx 4)))

(fn 2Dto1D
  (params (X :type Integer) (Z :type Integer))
  (return (+ X (* Z 4))))

(fn 2DtoTransform
  (params (X :type Integer) (Z :type Integer))
  (return (Math|Transform|MakeTransform (Math|Vector|MakeVector (Math|Conversions|ToFloat(Integer) (- (* X 182) 273)) 0.0 (Math|Conversions|ToFloat(Integer) (- (* Z 182) 273))))))